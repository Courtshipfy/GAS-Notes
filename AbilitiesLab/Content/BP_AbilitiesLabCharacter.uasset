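; BP_AbilitiesLabCharacter is a test character for the Gameplay Ability System with a world health bar and a self-damage ability.
; On BeginPlay it passes the health attribute set from its ability system component to the WBP_HealthBarWorld widget, then grants GA_DamageSelf.
; Pressing X tries to activate that ability by class, with remote activation allowed.
; An unconnected node that applies GE_Health_Minus15 directly never runs.
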(event `Key|X`
  (params (Key :type "Key Structure"))
  (:`Pressed`
    (`AbilitySystemComponent.TryActivateAbilityByClass` (`self.LabAbilitySystemComp`) "/Game/GA_DamageSelf.GA_DamageSelf_C" true)))

(event `self.ReceiveBeginPlay`
  (`|ExecutionSequence`
    (:`then_0`
      (bind _aswbp_health_bar_world (cast `/Game/WBP_HealthBarWorld` (`WidgetComponent.GetWidget` (`self.Widget`))))
      (bind _returnvalue (`AbilitySystemComponent.GetAttributeSet` (`self.LabAbilitySystemComp`) "/Script/AbilitiesLab.LabHealthAttributeSet"))
      (`/Game/WBP_HealthBarWorld.SetHealthAttributeSet` _aswbp_health_bar_world _returnvalue))
    (:`then_1`
      (`AbilitySystemComponent.K2_GiveAbility` (`self.LabAbilitySystemComp`) "/Game/GA_DamageSelf.GA_DamageSelf_C" 0 -1))))

(fn `UserConstructionScript`)